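; CameraCharacter is a Character Blueprint that provides yaw-relative movement and sets up player stats and UI.
; MoveForward and MoveRight axis inputs add movement along the forward and right vectors of the control rotation's yaw, scaled by a movement factor.
; On BeginPlay, it initializes HP and FP on HealthStats, then creates a UI widget and adds it to the viewport.
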(event `InputAxis|MoveForward`
  (params (AxisValue :type "Float (single-precision)"))
  ;[1 1 1] Move camera
  (`self.AddMovementInput` (`KismetMathLibrary.GetForwardVector` (`KismetMathLibrary.MakeRotator` 0.0 0.0 (.yaw (`self.GetControlRotation`)))) (* AxisValue (`self.MovemetInputFac`))))

(event `InputAxis|MoveRight`
  (params (AxisValue :type "Float (single-precision)"))
  ;[1 1 1] Move camera
  (`self.AddMovementInput` (`KismetMathLibrary.GetRightVector` (`KismetMathLibrary.MakeRotator` 0.0 0.0 (.yaw (`self.GetControlRotation`)))) (* AxisValue (`self.MovemetInputFac`))))

(event `self.ReceiveBeginPlay`
  (`|ExecutionSequence`
    (:`then_0`
      (`/Game/Blueprints/HealthStats.Set HP and FP` (`self.HealthStats`) 100.0 80.0 100.0 60.0))
    (:`then_1`
      (bind _returnvalue (`|CreateWidget` "/Game/Blueprints/UI/UI.UI_C"))
      (`UserWidget.AddToViewport` _returnvalue 0))))

(fn `UserConstructionScript`)