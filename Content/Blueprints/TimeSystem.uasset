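; Day/night cycle Blueprint that keeps game time and drives the sun and sky lighting.
; The SunMovement timeline, rate-scaled by TimeSpeed, supplies clock seconds, directional light rotation and both light intensities each tick.
; TimeSystem builds a Timespan, counting days through flags that detect the hour 23-to-0 rollover.
; Tick also prints debug time and periodically recaptures the skylight, while the sky sphere update is unconnected.
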(event `self.ReceiveTick`
  (params (DeltaSeconds :type "Float (single-precision)"))
  (`self.TimeSystem`)
  (set `self.MovementSec` (stale `self.ReceiveBeginPlay` _time))
  (`self.K2_SetActorRotation` (`self.DirLight`) (`KismetMathLibrary.MakeRotator` 0.0 (stale `self.ReceiveBeginPlay` _y_sun_pitch) (stale `self.ReceiveBeginPlay` _z_sun_yaw)) false)
  (`SkyLightComponent.SetIntensity` (`SkyLight.LightComponent` (`self.SkyLight`)) (stale `self.ReceiveBeginPlay` _sky_light_intensity))
  (`|ExecutionSequence`
    (:`then_0`
      (`LightComponent.SetIntensity` (`Light.LightComponent` (`self.DirLight`)) (stale `self.ReceiveBeginPlay` _dir_light_intensity))
      (`self.DisplayTime`))
    (:`then_1`
      (set `self.Timer` (+ (`GameplayStatics.GetWorldDeltaSeconds`) (`self.Timer`)))
      (if (>= (`self.Timer`) 3.0)
        (set `self.Timer` 0.0)
        (`SkyLightComponent.RecaptureSky` (`SkyLight.LightComponent` (`self.SkyLight`)))
        (`KismetSystemLibrary.PrintString` "Sky was update" true true (struct :`G` 0.004828 :`B` 1.0 :`A` 1.0) 1.5)))))

(event `self.ReceiveBeginPlay`
  (bind (_direction _y_sun_pitch _z_sun_yaw _time _sky_light_intensity _dir_light_intensity) (`Timeline|Sun Movement` :`NewTime` 6.0)))

(fn `DayTickSystem`
  (bind (_time_days _time_hours) (`KismetMathLibrary.BreakTimespan` (`self.Time`)))
  (bind (_time_days_2 _time_hours_2) (`KismetMathLibrary.BreakTimespan` (`self.Time`)))
  (bind (_time_days_3 _time_hours_3) (`KismetMathLibrary.BreakTimespan` (`self.Time`)))
  (`|ExecutionSequence`
    (:`then_0`
      (if (== _time_hours_3 23)
        (set `self.23` true)))
    (:`then_1`
      (if (== _time_hours 0)
        (set `self.00` true)))
    (:`then_2`
      (if (and (`self.23`) (`self.00`))
        (set `self.Day` (+ (`self.Day`) 1))
        (set `self.23` false)
        (set `self.00` false)))
    (:`then_3`
      (if (and (>= _time_hours_2 1) (<= _time_hours_2 23))
        (set `self.00` false)))))

(fn `DisplayTime`
  (bind (_days _hours _minutes _seconds) (`KismetMathLibrary.BreakTimespan` (`self.Time`)))
  (`KismetSystemLibrary.PrintString` (`KismetTextLibrary.Conv_TextToString` (`|FormatText` "Day: {day} {h}:{m}:{s}" (`KismetTextLibrary.Conv_IntToText` _days false true 2) (`KismetTextLibrary.Conv_IntToText` _hours false true 2) (`KismetTextLibrary.Conv_IntToText` _minutes false true 2) (`KismetTextLibrary.Conv_IntToText` _seconds false true 2))) true true (struct :`G` 0.66 :`B` 1.0 :`A` 1.0) 0.0)
  (`KismetSystemLibrary.PrintString` (`KismetStringLibrary.Concat_StrStr` "23" (`KismetStringLibrary.Conv_BoolToString` (`self.23`))) true true (struct :`R` 1.0 :`G` 0.087066 :`A` 1.0) 0.0)
  (`KismetSystemLibrary.PrintString` (`KismetStringLibrary.Concat_StrStr` "00" (`KismetStringLibrary.Conv_BoolToString` (`self.00`))) true true (struct :`R` 0.101557 :`G` 1.0 :`A` 1.0) 0.0))

(fn `RecapturingSky`)

(fn `TimeSystem`
  (`self.DayTickSystem`)
  (set `self.Time` (`KismetMathLibrary.MakeTimespan` (`self.Day`) 0 0 (`KismetMathLibrary.FTrunc` (`self.MovementSec`))))
  (return))

(fn `UserConstructionScript`
  (`TimelineComponent.SetPlayRate` (`self.Sun Movement`) (`self.TimeSpeed`)))