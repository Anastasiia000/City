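; Player character for a life-sim style game with a movable camera and decaying health, hunger and mood stats.
; Axis input and mouse screen-edge scrolling add yaw-relative movement, gated by an alive-check macro on the HealthStats death flag.
; BeginPlay seeds HealthStats with the stats, including money and smart points, and adds the UI widget.
; Tick lowers health, food and fun by fixed per-frame amounts, syncing them back to HealthStats.
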(event `InputAxisKey|MouseX`
  (params (AxisValue :type "Float (single-precision)"))
  (bind _returnvalue (/ (`PlayerController.GetMousePosition` (`GameplayStatics.GetPlayerController` 0)) (`KismetMathLibrary.BreakVector2D` (`WidgetLayoutLibrary.GetViewportSize`))))
  (bind _returnvalue_2 (`KismetMathLibrary.GetRightVector` (`KismetMathLibrary.MakeRotator` 0.0 0.0 (.yaw (`self.GetControlRotation`)))))
  ;[1 1 1] Move camera with mouse - edge scrolling
  (if (> _returnvalue 0.95)
    (`self.Is Alive? Can do?`
      (:`Can do`
        (`KismetSystemLibrary.PrintString` "right")
        (`self.AddMovementInput` _returnvalue_2)))
    (elif (< _returnvalue 0.05)
      (`self.Is Alive? Can do?`
        (:`Can do`
          (`KismetSystemLibrary.PrintString` "left")
          (`self.AddMovementInput` _returnvalue_2 -1.0))))))

(event `InputAxisKey|MouseY`
  (params (AxisValue :type "Float (single-precision)"))
  (bind _returnvalue (/ (`.LocationY` (`PlayerController.GetMousePosition` (`GameplayStatics.GetPlayerController` 0))) (`.Y` (`KismetMathLibrary.BreakVector2D` (`WidgetLayoutLibrary.GetViewportSize`)))))
  (bind _returnvalue_2 (`KismetMathLibrary.GetForwardVector` (`KismetMathLibrary.MakeRotator` 0.0 0.0 (.yaw (`self.GetControlRotation`)))))
  ;[1 1 1] Move camera with mouse - edge scrolling
  (if (> _returnvalue 0.95)
    (`self.Is Alive? Can do?`
      (:`Can do`
        (`KismetSystemLibrary.PrintString` "bottom")
        (`self.AddMovementInput` _returnvalue_2 -1.0)))
    (elif (< _returnvalue 0.05)
      (`self.Is Alive? Can do?`
        (:`Can do`
          (`KismetSystemLibrary.PrintString` "top")
          (`self.AddMovementInput` _returnvalue_2))))))

(event `InputAxis|MoveForward`
  (params (AxisValue :type "Float (single-precision)"))
  ;[1 1 1] Move camera
  (`self.Is Alive? Can do?`
    (:`Can do`
      (`self.AddMovementInput` (`KismetMathLibrary.GetForwardVector` (`KismetMathLibrary.MakeRotator` 0.0 0.0 (.yaw (`self.GetControlRotation`)))) (* AxisValue (`self.MovemetInputFac`))))))

(event `InputAxis|MoveRight`
  (params (AxisValue :type "Float (single-precision)"))
  ;[1 1 1] Move camera
  (`self.Is Alive? Can do?`
    (:`Can do`
      (`self.AddMovementInput` (`KismetMathLibrary.GetRightVector` (`KismetMathLibrary.MakeRotator` 0.0 0.0 (.yaw (`self.GetControlRotation`)))) (* AxisValue (`self.MovemetInputFac`))))))

(event `self.ReceiveBeginPlay`
  ;[1 1 1] Set health stats
  (`|ExecutionSequence`
    (:`then_0`
      (`/Game/Blueprints/HealthStats.Set HP and FP` (`self.HealthStats`) (`self.Health Points`) (`self.Funny Points`) (`self.Food Points`) (`self.Money`) (`self.Smart`)))
    (:`then_1`
      (bind _returnvalue (`|CreateWidget` "/Game/Blueprints/UI/UI.UI_C"))
      (bind _output_get (set `self.UI` _returnvalue))
      (`UserWidget.AddToViewport` _output_get 0))))

(event `self.ReceiveTick`
  (params (DeltaSeconds :type "Float (single-precision)"))
  ;[1 1 1] Change HealthStats
  (`|ExecutionSequence`
    (:`then_0`
      (bind _current_hp (`/Game/Blueprints/HealthStats.ChangeHealth` (`self.HealthStats`) -0.003))
      (set `self.Health Points` _current_hp))
    (:`then_1`
      (bind _foodpoins (`/Game/Blueprints/HealthStats.ChangeHunger` (`self.HealthStats`) -0.03))
      (set `self.Food Points` _foodpoins))
    (:`then_2`
      (bind _funnypoins (`/Game/Blueprints/HealthStats.ChangeMood` (`self.HealthStats`) -0.009))
      (set `self.Funny Points` _funnypoins)))
  (`/Game/Blueprints/HealthStats.Set HP and FP` (`self.HealthStats`) (`self.Health Points`) (`self.Funny Points`) (`self.Food Points`) (`self.Money`) (`self.Smart`)))

(fn `UserConstructionScript`)