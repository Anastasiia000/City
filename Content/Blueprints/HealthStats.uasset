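; HealthStats tracks the player's health, mood, food, money and smart points, and triggers the death and happy-end outcomes.
; Change functions clamp health, mood and food, refuse overspending, and flag death on depleted health or food; getters format values for the HUD.
; Tick polls for low-health death, the money goal and late-night sleep, which locks movement, routing events to PlayerCharacter's UI.
; The hunger alert check is never called.
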(event `HappyEnd`
  ;[1 1 1] call happyend
  (`/Game/Blueprints/UI/UI.HappyEndEvent` (`/Game/Blueprints/PlayerCharacter.UI` (cast `/Game/Blueprints/PlayerCharacter` (`GameplayStatics.GetPlayerCharacter` 0) :!pure true))))

(event `Death`
  ;[1 1 1] call death
  (set `self.Is Death?` true)
  (`/Game/Blueprints/UI/UI.DeathScreenEvent` (`/Game/Blueprints/PlayerCharacter.UI` (cast `/Game/Blueprints/PlayerCharacter` (`GameplayStatics.GetPlayerCharacter` 0) :!pure true))))

(event `self.ReceiveTick`
  (params (DeltaSeconds :type "Float (single-precision)"))
  ;[1 1 1] eventTick
  (`|ExecutionSequence`
    (:`then_1`
      (`self.Call "Death" Event When HP = 0`))
    (:`then_2`
      (`self.Call "Sleep"`))
    (:`then_3`
      (`self.Call "HappyEnd" Event When Money >= 10000`))))

(event `Hungry`
  ;[1 1 1] call hungryEvent
  (`/Game/Blueprints/UI/GameStore/Attention/Attention.HungryEvent` (`/Game/Blueprints/UI/UI.Attention` (`/Game/Blueprints/PlayerCharacter.UI` (cast `/Game/Blueprints/PlayerCharacter` (`GameplayStatics.GetPlayerCharacter` 0) :!pure true)))))

(event `Sleep`
  ;[1 1 1] call sleepEvent
  (`/Game/Blueprints/UI/GameStore/Attention/Attention.SleepEvent` (`/Game/Blueprints/UI/UI.Attention` (`/Game/Blueprints/PlayerCharacter.UI` (cast `/Game/Blueprints/PlayerCharacter` (`GameplayStatics.GetPlayerCharacter` 0) :!pure true)))))

(fn `ChangeHealth`
  (params (Value :type "Float (double-precision)"))
  (returns (`current HP` :type "Float (double-precision)"))
  (if (not (`self.Is Death?`))
    (if (and (< (`self.Current HealthPoints`) 1.0) true)
      (set `self.Is Death?` true)
      (else
        (bind _output_get (set `self.Current HealthPoints` (`KismetMathLibrary.FMax` (`KismetMathLibrary.FMin` (+ (`self.Current HealthPoints`) Value) 100.0))))))
    (return _output_get)))

(fn `ChangeHunger`
  (params (Value :type "Float (double-precision)"))
  (returns (FoodPoins :type "Float (double-precision)"))
  (if (not (`self.Is Death?`))
    (if (<= (`self.Current FoodPoins`) 0.0)
      (set `self.Is Death?` true)
      (else
        (bind _output_get (set `self.Current FoodPoins` (`KismetMathLibrary.FMax` (`KismetMathLibrary.FMin` (+ (`self.Current FoodPoins`) Value) 100.0))))))
    (return _output_get)))

(fn `ChangeMoney`
  (params (Value :type "Float (double-precision)"))
  (returns (Money :type "Float (double-precision)") (HaveWeMoney :type Boolean))
  (bind _returnvalue (+ (`self.Current Money`) Value))
  (bind _returnvalue_2 (>= _returnvalue 0.0))
  (if (not (`self.Is Death?`))
    (if _returnvalue_2
      (bind _output_get (set `self.Current Money` _returnvalue))
      (else
        (`KismetSystemLibrary.PrintString` "not enouth money")))
    (return _output_get _returnvalue_2)))

(fn `ChangeMood`
  (params (Value :type "Float (double-precision)"))
  (returns (FunnyPoins :type "Float (double-precision)"))
  (if (`self.Is Death?`)
    _
    (elif (> (`self.Current FunnyPoints`) 0.0)
      (bind _output_get (set `self.Current FunnyPoints` (`KismetMathLibrary.FMax` (`KismetMathLibrary.FMin` (+ (`self.Current FunnyPoints`) Value) 100.0))))
      (return _output_get))))

(fn `Get Stats For HUD`
  (returns (`Current HP` :type Text) (`HP Progress Bar` :type "Float (double-precision)") (`Current FP` :type Text) (`FP Progress Bar` :type "Float (double-precision)") (`Current Food` :type Text) (`Food Progres Bar` :type "Float (double-precision)") (Money :type Text))
  (return (`KismetTextLibrary.Conv_IntToText` (`KismetMathLibrary.FTrunc` (`self.Current HealthPoints`))) (`KismetMathLibrary.NormalizeToRange` (`self.Current HealthPoints`) 0.0 100.0) (`KismetTextLibrary.Conv_IntToText` (`KismetMathLibrary.FTrunc` (`self.Current FunnyPoints`))) (`KismetMathLibrary.NormalizeToRange` (`self.Current FunnyPoints`) 0.0 100.0) (`KismetTextLibrary.Conv_IntToText` (`KismetMathLibrary.FTrunc` (`self.Current FoodPoins`))) (`KismetMathLibrary.NormalizeToRange` (`self.Current FoodPoins`) 0.0 100.0) (`KismetTextLibrary.Conv_IntToText` (`KismetMathLibrary.FTrunc` (`self.Current Money`)))))

(fn `Get Status For SmartPoints`
  (returns (SmartPoints :type Text))
  (return (`KismetTextLibrary.Conv_IntToText` (`KismetMathLibrary.FTrunc` (`self.Current SmartPoints`)))))

(fn `Set HP and FP`
  (params (`Set HealthPoints` :type "Float (double-precision)") (`Set FunnyPoints` :type "Float (double-precision)") (`Set FoodPoints` :type "Float (double-precision)") (`Set Money` :type "Float (double-precision)") (`Set SmartPoints` :type "Float (double-precision)"))
  (set `self.Current HealthPoints` `Set HealthPoints`)
  (set `self.Current FunnyPoints` `Set FunnyPoints`)
  (set `self.Current FoodPoins` `Set FoodPoints`)
  (set `self.Current Money` `Set Money`)
  (set `self.Current SmartPoints` `Set SmartPoints`))