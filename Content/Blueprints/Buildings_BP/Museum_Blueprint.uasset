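; Museum building actor that shows an interaction prompt and museum UI when something enters its trigger box.
; Entering the trigger shows the F component and adds a BTNmuseum widget to the viewport.
; Leaving hides F, removes the widget and clears IsTimeStop on the first TimeSystem actor found, so any paused time resumes.
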(event `self.ReceiveBeginPlay`
  (`SceneComponent.SetVisibility` (`self.f`) false false))

(event `self.ReceiveActorBeginOverlap`
  (params (OtherActor :type "Actor Object Reference")))

(event `self.triggerBox.OnComponentBeginOverlap`
  (params (OverlappedComponent :type "PrimitiveComponent Object Reference") (OtherActor :type "Actor Object Reference") (OtherComp :type "PrimitiveComponent Object Reference") (OtherBodyIndex :type Integer) (bFromSweep :type Boolean) (SweepResult :type "HitResult Structure (by ref)"))
  (`SceneComponent.SetVisibility` (`self.f`) true false)
  (bind _returnvalue (`|CreateWidget` "/Game/Blueprints/UI/GameStore/UI_ButtonClick/BTNmuseum.BTNmuseum_C"))
  (bind _output_get (set `self.UI` _returnvalue))
  (`UserWidget.AddToViewport` _output_get 0))

(event `self.triggerBox.OnComponentEndOverlap`
  (params (OverlappedComponent :type "PrimitiveComponent Object Reference") (OtherActor :type "Actor Object Reference") (OtherComp :type "PrimitiveComponent Object Reference") (OtherBodyIndex :type Integer))
  (`SceneComponent.SetVisibility` (`self.f`) false false)
  (`Widget.RemoveFromParent` (`self.UI`))
  (bind _outactors (`GameplayStatics.GetAllActorsOfClass` "/Game/Blueprints/TimeSystem.TimeSystem_C"))
  (set `/Game/Blueprints/TimeSystem.IsTimeStop` false (`|GetArrayItem` _outactors)))

(fn `UserConstructionScript`)